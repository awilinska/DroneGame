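; BP_SmallSphere is a drifting, timed collectible that raises the BP_DroneGameMode score when a Pawn overlaps it.
; It scales in on BeginPlay, picks a random spin, then each Tick moves along its constantly rotating forward vector.
; Lifetime expiry or a Pawn overlap calls WinkOut, whose timeline, gated by IsWinking, rescales the mesh and destroys the actor when finished.
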(event `self.ReceiveBeginPlay`
  (`self.WinkIn`)
  (`self.InitializeDeltaRotation`)
  ; Start WinkOut Timeline
  (`KismetSystemLibrary.K2_SetTimerDelegate` (delegate `WinkOut`) (`self.Lifetime`))
  ; Handle Overlap
  (add `PrimitiveComponent.OnComponentBeginOverlap` (`self.SphereVolume`) (delegate `OnSphereOverlap`)))

(event `WinkOut`
  ; Start WinkOut Timeline
  (if (`self.IsWinking`)
    (set `self.IsWinking` true)
    (bind (_direction _scale) (`Timeline|WinkOutTimeline`)
      (:`Update`
        (`self.ScaleSphere` _scale))
      (:`Finished`
        (`self.K2_DestroyActor`)))))

(event `OnSphereOverlap`
  (params (OverlappedComponent :type "PrimitiveComponent Object Reference") (OtherActor :type "Actor Object Reference") (OtherComp :type "PrimitiveComponent Object Reference") (OtherBodyIndex :type Integer) (bFromSweep :type Boolean) (SweepResult :type "HitResult Structure (by ref)"))
  ; Handle Overlap
  (if (`GameplayStatics.ObjectIsA` OtherActor "/Script/Engine.Pawn")
    (bind _asbp_drone_game_mode (cast `/Game/Blueprints/Game/BP_DroneGameMode` (`GameplayStatics.GetGameMode`)))
    (`/Game/Blueprints/Game/BP_DroneGameMode.IncrementScore` _asbp_drone_game_mode)
    (`self.WinkOut`)))

(event `WinkIn`
  ; WinkIn
  (bind (_direction _scale) (`Timeline|WinkIn Timeline`)
    (:`Update`
      (`SceneComponent.SetWorldScale3D` (`self.SM_SmallSphere`) _scale))))

(event `self.ReceiveTick`
  (params (DeltaSeconds :type "Float (single-precision)"))
  ; Update Location and Rotation
  (`self.UpdateLocation` DeltaSeconds)
  (`self.UpdateRotation`))

(fn `InitializeDeltaRotation`
  (set `self.Delta Rotation` (* (`KismetMathLibrary.RandomRotator` false) (`self.RotationScaleFactor`))))

(fn `ScaleSphere`
  (params (Scale :type "Float (single-precision)"))
  (`SceneComponent.SetWorldScale3D` (`self.SM_SmallSphere`) (`KismetMathLibrary.MakeVector` Scale Scale Scale)))

(fn `UpdateLocation`
  (params (DeltaSeconds :type "Float (single-precision)"))
  (`self.K2_AddActorWorldOffset` (* (`self.GetActorForwardVector`) (* DeltaSeconds (`self.Speed`)))))

(fn `UpdateRotation`
  (`self.K2_AddActorWorldRotation` (* (`self.Delta Rotation`) (`GameplayStatics.GetWorldDeltaSeconds`))))

(fn `UserConstructionScript`)