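; BP_SphereSpawner is an actor that periodically spawns BP_SmallSphere actors at random points within a spherical radius around itself.
; BeginPlay starts a looping timer on SpawnTime and spawns one immediately, each with a random rotation.
; Spawn points come from a random direction scaled by a uniform random distance, so they cluster toward the center.
; Tick draws a debug sphere showing the spawn radius.
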(event `self.ReceiveBeginPlay`
  ; Start Sphere Spawn Timer
  (`KismetSystemLibrary.K2_SetTimerDelegate` (delegate `SpawnSmallSphere`) (`self.SpawnTime`) true)
  (`self.SpawnSmallSphere`))

(event `SpawnSmallSphere`
  ; Start Sphere Spawn Timer
  (`|SpawnActorFromClass` "/Game/Blueprints/SmallSphere/BP_SmallSphere.BP_SmallSphere_C" (`KismetMathLibrary.MakeTransform` (`self.GetRandomPointInSphereRadius`) (`KismetMathLibrary.RandomRotator` false)) "Undefined" "MultiplyWithRoot" null null))

(event `self.ReceiveTick`
  (params (DeltaSeconds :type "Float (single-precision)"))
  (`KismetSystemLibrary.DrawDebugSphere` (`self.K2_GetActorLocation`) (`self.SpawnRadius`)))

(fn `GetRandomPointInSphereRadius`
  (returns (RandomPoint :type "Vector Structure"))
  (return (+ (`self.K2_GetActorLocation`) (* (`KismetMathLibrary.GetForwardVector` (`KismetMathLibrary.RandomRotator` false)) (`KismetMathLibrary.RandomFloatInRange` 0.0 (`self.SpawnRadius`))))))

(fn `UserConstructionScript`)